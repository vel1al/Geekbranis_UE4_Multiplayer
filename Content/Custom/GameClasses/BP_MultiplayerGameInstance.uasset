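; BP_MultiplayerGameInstance is a game instance that hosts, finds and joins multiplayer sessions.
; CreateGame creates a session with a player limit and LAN option, then opens the chosen map as a listen server.
; UpdateServerList runs a LAN-only search and caches the results for GetSessionsList, and JoinGame joins a given result.
; Network and travel error handlers print the failure type on screen.
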(event `CreateGame`
  (params (MaxPlayersCount :type Integer) (LAN :type Boolean) (MapName :type Name))
  (`CreateSessionCallbackProxy.CreateSession` (`GameplayStatics.GetPlayerController` 0) MaxPlayersCount LAN
    (:`OnSuccess`
      (`GameplayStatics.OpenLevel` MapName true "listen"))))

(event `UpdateServerList`
  (bind _results (`FindSessionsCallbackProxy.FindSessions` (`GameplayStatics.GetPlayerController` 0) 20 true)
    (:`OnSuccess`
      (set `self.SessionsList` _results))))

(event `JoinGame`
  (params (Session :type "BlueprintSessionResult Structure"))
  (`JoinSessionCallbackProxy.JoinSession` (`GameplayStatics.GetPlayerController` 0) Session))

(event `self.HandleNetworkError`
  (params (FailureType :type "ENetworkFailure Enum" :default "NetDriverAlreadyExists") (bIsServer :type Boolean))
  (`KismetSystemLibrary.PrintString` (`KismetStringLibrary.Concat_StrStr` "NetworkError:" (`|GetEnumeratorNameAsString` FailureType) " .On Server? " (`KismetStringLibrary.Conv_BoolToString` bIsServer)) true true (struct :`G` 0.66 :`B` 1.0 :`A` 1.0) 10.0))

(event `self.HandleTravelError`
  (params (FailureType :type "ETravelFailure Enum" :default "NoLevel"))
  (`KismetSystemLibrary.PrintString` (`KismetStringLibrary.Concat_StrStr` "TravelError: " (`|GetEnumeratorNameAsString` FailureType)) true true (struct :`G` 0.66 :`B` 1.0 :`A` 1.0) 10.0))

(fn `GetSessionsList`
  (returns (`Sessions List` :type "Array of BlueprintSessionResult Structure"))
  (return (`self.SessionsList`)))