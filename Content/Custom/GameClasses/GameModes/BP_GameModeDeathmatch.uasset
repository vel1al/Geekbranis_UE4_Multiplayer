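; BP_GameModeDeathmatch is the deathmatch game mode, which registers joining and leaving players in a single Team1 array.
; On PostLogin it casts to BP_PlayerController, assigns team zero and a player number equal to the current array length, then adds the controller.
; A failed cast prints an error.
; OnLogout removes the controller without renumbering the remaining players.
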(event `self.K2_PostLogin`
  (params (NewPlayer :type "PlayerController Object Reference"))
  (bind _team1 (`self.Team1`))
  (bind _asbp_player_controller (cast `/Game/Custom/Character/BP_PlayerController` NewPlayer)
    (:`then`
      (`/Game/Custom/Character/BP_PlayerController.SetTeamNumber` _asbp_player_controller 0)
      (`/Game/Custom/Character/BP_PlayerController.SetPlayerNumber` _asbp_player_controller (`KismetMathLibrary.Conv_IntToByte` (`KismetArrayLibrary.Array_Length` _team1)))
      (`KismetArrayLibrary.Array_Add` _team1 _asbp_player_controller))
    (:`CastFailed`
      (`KismetSystemLibrary.PrintString` "PostLogin Error"))))

(event `self.K2_OnLogout`
  (params (ExitingController :type "Controller Object Reference"))
  (bind _asbp_player_controller (cast `/Game/Custom/Character/BP_PlayerController` ExitingController))
  (`KismetArrayLibrary.Array_RemoveItem` (`self.Team1`) _asbp_player_controller))

(fn `UserConstructionScript`)