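; BP_HealthComponent is a character health component that stores a current health value and exposes it through set, get, add and damage operations.
; TakeDamage returns true for damage at or above current health without changing it; otherwise it subtracts the damage and returns false.
; AddHealth ignores negative values and applies no upper limit, while SetHealth assigns the value directly.
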(event `SetHealth`
  (params (Value :type "Float (double-precision)"))
  (set `self.CurrentHealth` Value))

(fn `AddHealth`
  (params (Value :type "Float (double-precision)"))
  (if (not (< Value 0.0))
    (set `self.CurrentHealth` (+ Value (`self.CurrentHealth`)))))

(fn `GetHealth`
  (returns (Health :type "Float (double-precision)"))
  (return (`self.CurrentHealth`)))

(fn `TakeDamage`
  (params (Value :type "Float (double-precision)"))
  (returns (IsDead :type Boolean))
  (bind _currenthealth (`self.CurrentHealth`))
  (if (>= Value _currenthealth)
    (return true)
    (else
      (set `self.CurrentHealth` (- _currenthealth Value))
      (return false))))