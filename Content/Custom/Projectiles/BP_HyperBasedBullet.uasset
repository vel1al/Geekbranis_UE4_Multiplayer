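; Projectile base for an explosive bullet that flies forward at a set speed and destroys itself when its lifetime timer ends.
; Movement, collision and destruction route through Server-named events, with Tick offsetting the actor without sweep.
; Capsule overlaps, except with same-owner bullets of this class, run a debug-drawn multi capsule trace that ignores the owner.
; The trace damages characters in the blast radius, then the bullet spawns an explosion emitter and destroys itself.
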(event `self.ReceiveBeginPlay`
  (`KismetSystemLibrary.K2_SetTimerDelegate` (delegate `BulletLifeEnd`) (`self.LiveTime`)))

(event `BulletLifeEnd`
  (`self.ServerBulletLifeEnd`))

(event `ServerBulletLifeEnd`
  (`self.K2_DestroyActor`))

(event `self.ReceiveTick`
  (params (DeltaSeconds :type "Float (single-precision)"))
  (`self.ServerMoveBullet` DeltaSeconds))

(event `ServerMoveBullet`
  (params (DeltaSeconds :type "Float (double-precision)"))
  (`self.K2_AddActorWorldOffset` (* (`self.GetActorForwardVector`) (* DeltaSeconds (`self.FlySpeed`)))))

(event `self.Capsule.OnComponentBeginOverlap`
  (params (OverlappedComponent :type "PrimitiveComponent Object Reference") (OtherActor :type "Actor Object Reference") (OtherComp :type "PrimitiveComponent Object Reference") (OtherBodyIndex :type Integer) (bFromSweep :type Boolean) (SweepResult :type "HitResult Structure (by ref)"))
  (`self.ServerCollisionBegin` OtherActor (`self.K2_GetActorLocation`)))

(event `ServerCollisionBegin`
  (params (OverllapingActor :type "Actor Object Reference") (OverllapLocation :type "Vector Structure"))
  (bind _asbp_hyper_based_bullet (cast `/Game/Custom/Projectiles/BP_HyperBasedBullet` OverllapingActor)
    (:`then`
      (if (!= (`self.GetOwner` _asbp_hyper_based_bullet) (`self.GetOwner`))
        (bind _outhits (`KismetSystemLibrary.CapsuleTraceMulti` OverllapLocation OverllapLocation (`self.BlastRadius`) 0.0 "TraceTypeQuery1" false (`|MakeArray` (`self.GetOwner`)) "Persistent" :!label _label))
        (for _array_element _outhits
          (bind _asbp_default_character (cast `/Game/Custom/Character/BP_DefaultCharacter` (`.HitActor` (`GameplayStatics.BreakHitResult` _array_element))))
          (`/Game/Custom/Character/BP_DefaultCharacter.TakeDamage` _asbp_default_character (`self.Damage`)))
        (`self.ExplosionEffect` (`self.K2_GetActorLocation`))
        (`self.ServerBulletLifeEnd`)))
    (:`CastFailed`
      (goto _label))))

(event `ExplosionEffect`
  (params (Location :type "Vector Structure"))
  (`GameplayStatics.SpawnEmitterAtLocation` null Location))

(fn `UserConstructionScript`)